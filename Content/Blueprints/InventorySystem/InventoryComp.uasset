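; Inventory component that holds a resizable array of item slots and toggles a centered inventory window on the HUD canvas, switching between UI-only and game-only input.
; PrepareInventory sizes the array and refreshes each slot's item data from its class defaults on BeginPlay and when the window opens.
; AddItem fills partial stacks, recursing with any overflow, or takes an empty slot.
; InventoryQuery totals quantities to check for a required amount.
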(event EventBeginPlay
  (CallFunction|PrepareInventory))

(event EventTick
  (params (DeltaSeconds :type Float%20%28single-precision%29)))

(fn ToggleInventory
  (bind _returnvalue (Game|GetPlayerController 0))
  (bind _inventorywindow (Variables|Default|GetInventoryWindow)
    (:then
      (Widget|RemovefromParent _inventorywindow)
      (Variables|Default|SetInventoryWindow 0)
      (Input|SetInputModeGameOnly _returnvalue)
      (bind _asplayer (Utilities|Casting|CastToPlayer (Game|GetPlayerCharacter 0)))
      (Variables|/Game/Blueprints/Player.Player_C|SetOpeningContainer? _asplayer false))
    (:else
      (CallFunction|PrepareInventory)
      (bind _returnvalue_2 (UserInterface|CreateWidget "/Game/Blueprints/InventorySystem/InventoryUI/InventoryWindow.InventoryWindow_C" 0 self))
      (Variables|Default|SetInventoryWindow _returnvalue_2)
      (bind _asmy_player_controller (Utilities|Casting|CastToMyPlayerController _returnvalue))
      (bind _returnvalue_3 (Class|CanvasPanel|AddChildtoCanvas (Variables|/Game/Widgets/PlayerStatsHUD.PlayerStatsHUD_C|GetHUDCanvas (Variables|/Game/Blueprints/InventorySystem/InventoryUI/MyPlayerController.MyPlayerController_C|GetHUD%20Ref _asmy_player_controller)) (Variables|Default|GetInventoryWindow)))
      (Class|CanvasPanelSlot|SetAutoSize _returnvalue_3 true)
      (Class|CanvasPanelSlot|SetAlignment _returnvalue_3 "(X=0.500000,Y=0.500000)")
      (Class|CanvasPanelSlot|SetAnchors _returnvalue_3 (Utilities|Struct|MakeAnchors "(X=0.500000,Y=0.500000)" "(X=0.500000,Y=0.500000)"))
      (Class|CanvasPanelSlot|SetPosition _returnvalue_3 (Variables|Default|GetPosition))
      (Input|SetInputModeUIOnly (Game|GetPlayerController 0) (Variables|Default|GetInventoryWindow) "LockAlways"))))

(fn AddItem
  (params (ItemToAdd :type Slot%20Struct%20Structure))
  (if (.isstackable (.itemstructure ItemToAdd))
    (bind _stackindex (Utilities|HasPartialStack ItemToAdd)
      (:True
        (bind _addedtostack_ (CallFunction|AddtoStack ItemToAdd _stackindex))
        (return _addedtostack_))
      (:False
        _)))
  (bind _hascreated_ (CallFunction|CreateStack ItemToAdd))
  (return _hascreated_))

(fn PrepareInventory
  (bind _inventory (Variables|Default|GetInventory))
  (Utilities|Array|Resize _inventory (Variables|Default|GetNumSlots))
  (for (_array_element _array_index) _inventory
    (if (!= (.Class (Utilities|Struct|BreakItemStruct (.itemstructure _array_element))) 0)
      (Utilities|Array|SetArrayElem (Variables|Default|GetInventory) _array_index (Utilities|Struct|MakeSlotStruct (Utilities|GetClassDefaults (.Class (Utilities|Struct|BreakItemStruct (.itemstructure _array_element)))) (.quantity _array_element))))))

(fn CreateStack
  (params (ItemToAdd :type Slot%20Struct%20Structure))
  (bind _inventory (Variables|Default|GetInventory))
  (bind _array_element (Utilities|Array|ForEachLoopwithBreak (Variables|Default|GetInventory) :!label _label)
    (:LoopBody
      (if (<= (.quantity _array_element) 0)
        (LocalVariables|SetHasSpace true)
        (goto _label Break)))
    (:Completed
      (if (LocalVariables|GetHasSpace)
        (Utilities|Array|SetArrayElem _inventory (Utilities|Array|FindItem _inventory (Utilities|Struct|MakeSlotStruct "(Name_2_8A14B2174902239379402D90450B9836=NSLOCTEXT(\"[1C1CC151438033892B43DC94637379B2]\", \"CB6E295A473AF35F9EE262B53A5A692A\", \"NaN\"),isStackable_5_E5B90510421705A5CE2614847DB12A2B=True,Thumbnail_8_5334B7B24CBC804842F025B763A915E1=None,Description_11_1FF311BE44326502E2CDF08275E0452E=NSLOCTEXT(\"[1C1CC151438033892B43DC94637379B2]\", \"3677521041F389965D483DA447E839E1\", \"NaN\"),isConsumable_14_475AFE844A6A00B5C5686CA192D39101=True,MaxStackSize_17_15A16317470E3E93461978A3CC440E6C=4,ReplenishingValue_24_190A08854B114C37028DCABA1F0F6DCB=0.000000,Class_23_47A7ECE845D390F21F41519B608CC5C8=None,ItemMesh_27_D395D89445B58016B7E0A8BA21F6F730=None)")) ItemToAdd)
        (return (LocalVariables|GetHasSpace))
        (else
          (return false))))))

(fn AddtoStack
  (params (SlotStructure :type Slot%20Struct%20Structure) (SlotIndex :type Integer))
  (bind (_itemstructure _quantity) (Utilities|Struct|BreakSlotStruct SlotStructure))
  (bind _inventory (Variables|Default|GetInventory))
  (bind _maxstacksize (Utilities|Struct|BreakItemStruct (.itemstructure SlotStructure)))
  (bind _output (Utilities|Array|Get(acopy) _inventory SlotIndex))
  (bind _output_get (LocalVariables|SetCurrentStackQuantity (.quantity _output)))
  (if (> (+ _output_get _quantity) (.maxstacksize (.itemstructure _output)))
    (Utilities|Array|SetArrayElem (Variables|Default|GetInventory) SlotIndex (Utilities|Struct|MakeSlotStruct (.itemstructure SlotStructure) _maxstacksize))
    (CallFunction|AddItem (Utilities|Struct|MakeSlotStruct (.itemstructure SlotStructure) (- (.quantity SlotStructure) (- _maxstacksize (LocalVariables|GetCurrentStackQuantity)))))
    (else
      (Utilities|Array|SetArrayElem (Variables|Default|GetInventory) SlotIndex (Utilities|Struct|MakeSlotStruct _itemstructure (+ _output_get _quantity)))))
  (return true))

(fn InventoryQuery
  (params (QueryItem :type Item%20Class%20Reference) (QueryAmount :type Integer))
  (bind _array_element (Utilities|Array|ForEachLoopwithBreak (Variables|Default|GetInventory))
    (:LoopBody
      (if (== (.Class (Utilities|Struct|BreakItemStruct (.itemstructure _array_element))) QueryItem)
        (LocalVariables|SetRunningTotal (+ (.quantity _array_element) (LocalVariables|GetRunningTotal)))))
    (:Completed
      (if (>= (LocalVariables|GetRunningTotal) QueryAmount)
        (return true)))))