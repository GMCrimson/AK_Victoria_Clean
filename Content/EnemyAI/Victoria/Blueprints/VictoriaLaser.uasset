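; VictoriaLaser is the laser hazard for the Victoria enemy, changing the player's health repeatedly while the player is inside it.
; Hitbox begin and end overlaps with the Player toggle a Ticking flag.
; While that flag is set, Tick passes Damage to the player's ChangeHealth, using a Damaging flag and a short Delay to throttle hits to a fixed interval instead of every frame.
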(event OnComponentBeginOverlap(Hitbox)
  (params (OverlappedComponent :type Primitive%20Component%20Object%20Reference) (OtherActor :type Actor%20Object%20Reference) (OtherComp :type Primitive%20Component%20Object%20Reference) (OtherBodyIndex :type Integer) (bFromSweep :type Boolean) (SweepResult :type Hit%20Result%20Structure%20%28by%20ref%29))
  (Utilities|Casting|CastToPlayer OtherActor)
  (Variables|Default|SetTicking true))

(event OnComponentEndOverlap(Hitbox)
  (params (OverlappedComponent :type Primitive%20Component%20Object%20Reference) (OtherActor :type Actor%20Object%20Reference) (OtherComp :type Primitive%20Component%20Object%20Reference) (OtherBodyIndex :type Integer))
  (Utilities|Casting|CastToPlayer OtherActor)
  (Variables|Default|SetTicking false))

(event EventTick
  (params (DeltaSeconds :type Float%20%28single-precision%29))
  (if (Variables|Default|GetTicking)
    (if (not (Variables|Default|GetDamaging))
      (Variables|Default|SetDamaging true)
      (bind _asplayer (Utilities|Casting|CastToPlayer (Game|GetPlayerCharacter 0)))
      (Default|ChangeHealth _asplayer (Variables|Default|GetDamage))
      (Utilities|FlowControl|Delay 0.25)
      (Variables|Default|SetDamaging false))))

(fn ConstructionScript)